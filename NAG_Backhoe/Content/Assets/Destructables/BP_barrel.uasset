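; BP_barrel is a destructible barrel that costs the player budget when they hit it.
; The first component hit from the player pawn calls DecreaseBudget with the barrel's Cost on BP_ThirdPersonGameMode1.
; It then sets collision to ignore Pawns, plays a 2D sound and activates wood destruction and explosion particles.
; A FirstHit flag limits the reaction to one hit.
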(event OnComponentHit(barrel_cl)
  (params (HitComponent :type Primitive%20Component%20Object%20Reference) (OtherActor :type Actor%20Object%20Reference) (OtherComp :type Primitive%20Component%20Object%20Reference) (NormalImpulse :type Vector :default "0, 0, 0") (Hit :type Hit%20Result%20Structure%20%28by%20ref%29))
  (if (== OtherActor (Game|Player|GetPlayerPawn 0))
    (if (Variables|Default|GetfirstHit?)
      (Variables|Default|SetfirstHit? false)
      (bind _asbp_third_person_game_mode_1 (Utilities|Casting|CastToBP_ThirdPersonGameMode1 (Game|GetGameMode)))
      (Default|DecreaseBudget _asbp_third_person_game_mode_1 (Variables|Default|Getcost))
      (Collision|SetCollisionResponsetoChannel (Variables|Default|Getbarrel_cl) "ECC_Pawn" "ECR_Ignore")
      (Audio|PlaySound2D "/Game/Assets/Sound/SC_barrel.SC_barrel" 1.0 1.0 0.0 0 0)
      (Components|Activation|Activate (Variables|Default|GetP_Destruction_Wood) false))))

(event Custom|itemDestroyed)

(event EventBeginPlay)

(event Collision|EventActorBeginOverlap
  (params (OtherActor :type Actor%20Object%20Reference)))

(event EventTick
  (params (DeltaSeconds :type Float%20%28single-precision%29)))

(fn ConstructionScript)