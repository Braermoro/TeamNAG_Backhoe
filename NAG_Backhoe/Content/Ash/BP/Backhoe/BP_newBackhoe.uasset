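; Player-controllable backhoe Blueprint that drives the vehicle and aims its cabin and camera from axis inputs.
; Movement input follows the chassis forward vector rotated -90 degrees about Z, while turn input yaws the chassis.
; Look input yaws the cabin independently and pitches the spring arm, with camera rotation marked unfinished.
; It stores tread speed from capsule velocity and the turn value, though nothing here reads them.
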(event EventBeginPlay)

(event Collision|EventActorBeginOverlap
  (params (OtherActor :type Actor%20Object%20Reference)))

(event EventTick
  (params (DeltaSeconds :type Float%20%28single-precision%29)))

(event Input|AxisEvents|InputAxisLookUp
  (params (AxisValue :type Float%20%28single-precision%29))
  ;[1 1 1] General Movement
  ;;[1 1 1] CameraRotation(Unfinished)
  (Transformation|AddLocalRotation (Variables|Default|GetSpringArm) (Math|Rotator|MakeRotator 0.0 (* AxisValue (Variables|Default|GetLookUpSpeed)) 0.0) false false))

(event Input|AxisEvents|InputAxisMoveForward
  (params (AxisValue :type Float%20%28single-precision%29))
  ;[1 1 1] General Movement
  ;;[1 1 1] Movement&Rotation
  (Pawn|Input|AddMovementInput (Math|Vector|RotateVectorAroundAxis (Math|Vector|GetForwardVector (Variables|Default|GetChassis)) -9e+01 "0.000000,0.000000,1.000000") (* AxisValue (Variables|Default|GetMoveSpeed)) false)
  ;[1 1 1] Set current speed for each tread
  (Variables|Default|SetTreadSpeed (* (Math|Vector|VectorLength (Transformation|GetComponentVelocity (Variables|Collision|GetCapsuleComponent))) AxisValue)))

(event Input|AxisEvents|InputAxisLookRight
  (params (AxisValue :type Float%20%28single-precision%29))
  ;[1 1 1] General Movement
  ;;[1 1 1] CameraRotation(Unfinished)
  (Transformation|AddLocalRotation (Variables|Default|GetCabin) (Math|Rotator|MakeRotator 0.0 0.0 (* AxisValue (Variables|Default|GetRotationSpeed))) false false))

(event Input|AxisEvents|InputAxisRotateRight
  (params (AxisValue :type Float%20%28single-precision%29))
  ;[1 1 1] General Movement
  ;;[1 1 1] Movement&Rotation
  (Variables|Default|SetTurnValue AxisValue)
  (Transformation|AddLocalRotation (Variables|Default|GetChassis) (Math|Rotator|MakeRotator 0.0 0.0 (* AxisValue (Variables|Default|GetTurnSpeed))) false false))

(fn ConstructionScript)