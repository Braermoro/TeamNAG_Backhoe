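; BP_Backhoe is a drivable backhoe pawn with tread steering and an unfinished spring-arm orbit camera.
; Axis inputs rotate the tread pair and drive movement along its forward vector turned 90 degrees, while separate look inputs rotate the spring arm.
; Tick records tread speed from root velocity, and a hit handler shoves physics-simulating components using scaled vehicle velocity.
; Disconnected budget and barrel-damage nodes never run.
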(event Custom|CustomEvent
  (params (MyComp :type Primitive%20Component%20Object%20Reference) (Other :type Actor%20Object%20Reference) (OtherComp :type Primitive%20Component%20Object%20Reference) (bSelfMoved :type Boolean) (HitLocation :type Vector) (HitNormal :type Vector) (NormalImpulse :type Vector) (Hit :type Hit%20Result%20Structure%20%28by%20ref%29))
  (if (Physics|IsSimulatingPhysics OtherComp "None")
    (Physics|AddImpulseatLocation OtherComp (* (Transformation|GetVelocity) "100.000000,100.000000,100.000000") (Transformation|GetActorLocation) "None")))

(event EventTick
  (params (DeltaSeconds :type Float%20%28single-precision%29))
  ;[1 1 1] Set current speed for each tread
  (Variables|Default|SetTreadSpeed (Math|Vector|VectorLength (Transformation|GetComponentVelocity (Variables|Default|GetDefaultSceneRoot)))))

(event Input|AxisEvents|InputAxisLookUp
  (params (AxisValue :type Float%20%28single-precision%29))
  ;[1 1 1] General Movement
  ;;[1 1 1] CameraRotation(Unfinished)
  (Transformation|AddLocalRotation (Variables|Default|GetSpringArm) (Math|Rotator|MakeRotator 0.0 (* AxisValue (Variables|Default|GetLookUpSpeed)) 0.0) false false))

(event Input|AxisEvents|InputAxisMoveForward
  (params (AxisValue :type Float%20%28single-precision%29))
  ;[1 1 1] General Movement
  ;;[1 1 1] Movement&Rotation
  (Pawn|Input|AddMovementInput (Math|Vector|RotateVectorAroundAxis (Math|Vector|GetForwardVector (Variables|Default|GetTreadPair)) 9e+01 "0.000000,0.000000,1.000000") (* AxisValue (Variables|Default|GetMoveSpeed)) false))

(event Input|AxisEvents|InputAxisLookRight
  (params (AxisValue :type Float%20%28single-precision%29))
  ;[1 1 1] General Movement
  ;;[1 1 1] CameraRotation(Unfinished)
  (Transformation|AddLocalRotation (Variables|Default|GetSpringArm) (Math|Rotator|MakeRotator 0.0 0.0 (* AxisValue (Variables|Default|GetRotationSpeed))) false false))

(event Input|AxisEvents|InputAxisRotateRight
  (params (AxisValue :type Float%20%28single-precision%29))
  ;[1 1 1] General Movement
  ;;[1 1 1] Movement&Rotation
  (Variables|Default|SetTurnValue AxisValue) ; Used for rotating treads
  (Transformation|AddLocalRotation (Variables|Default|GetTreadPair) (Math|Rotator|MakeRotator 0.0 0.0 (* AxisValue (Variables|Default|GetTurnSpeed))) false false))

(fn ConstructionScript)